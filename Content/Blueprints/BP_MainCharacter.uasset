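; Player character Blueprint providing a flashlight toggle, object inspection, cursor-based focus mode, inventory display and pause menu.
; Inspection attaches an actor to InspectPoint for rotation and clamped distance adjustment, then restores its saved transform on exit.
; Inspect, focus and inventory states each swap Enhanced Input mapping contexts, with focus and inventory also switching input mode and cursor visibility.
; Inventory changes go out through a dispatcher call, while pausing spawns WBP_PauseMenu.
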(event `self.SwitchFlashlight`
  (bind _flashlight (`self.FlashLight`))
  ; Flashlight
  (if (`self.bFlashlightIsOn`)
    (`LightComponent.SetIntensity` _flashlight 0.0)
    (set `self.bFlashlightIsOn` false)
    (else
      (`LightComponent.SetIntensity` _flashlight (`self.FlashlightIntensity`))
      (set `self.bFlashlightIsOn` true))))

(event `self.Inspect`
  (params (ActorToInspect :type "Actor Object Reference"))
  (bind (_inspectableactororigintransform_location _inspectableactororigintransform_rotation _inspectableactororigintransform_scale) (`KismetMathLibrary.BreakTransform` (`self.InspectableActorOriginTransform`)))
  (bind _returnvalue (pcsubsystem `EnhancedInputLocalPlayerSubsystem` (`GameplayStatics.GetPlayerController` 0)))
  ; Interaction
  ;; Object inspection
  (bind _output_get (set `self.InspectingActor` ActorToInspect))
  (if (`self.bIsInInspection`)
    (`self.K2_DetachFromActor` (`self.InspectingActor`) "KeepRelative" "KeepRelative" "KeepRelative")
    (set `self.bIsInInspection` false)
    (`self.K2_SetActorTransform` (`self.InspectingActor`) (`KismetMathLibrary.MakeTransform` _inspectableactororigintransform_location _inspectableactororigintransform_rotation _inspectableactororigintransform_scale) false true)
    ;; Changing IMC
    (`EnhancedInputSubsystemInterface.ClearAllMappings` _returnvalue)
    (`EnhancedInputSubsystemInterface.AddMappingContext` _returnvalue "/Game/Input/Default/IMC_Default.IMC_Default" 0 (struct))
    ;; Reset variables for inspection
    (`SceneComponent.K2_SetRelativeLocation` (`self.InspectPoint`) (`KismetMathLibrary.MakeVector` (`self.DefaultPointX`)) false false)
    (else
      (set `self.InspectableActorOriginTransform` (`self.GetTransform` _output_get))
      (`self.K2_AttachToComponent` (`self.InspectingActor`) (`self.InspectPoint`) "None" "SnapToTarget" "KeepRelative" "KeepRelative" true)
      (set `self.bIsInInspection` true)
      (`EnhancedInputSubsystemInterface.ClearAllMappings` _returnvalue)
      (`EnhancedInputSubsystemInterface.AddMappingContext` _returnvalue "/Game/Input/Inspection/IMC_Inspect.IMC_Inspect" 0 (struct))
      (set `self.CurrentPointX` (`self.DefaultPointX`)))))

(event `self.RotateInspectableItem`
  (params (Value :type "InputActionValue Structure (by ref)"))
  (bind (_x _y) (`EnhancedInputLibrary.BreakInputActionValue` Value))
  ; Interaction
  ;; Inspect Actions
  (bind _inspectingactor (`self.InspectingActor`)
    (:`then`
      (`self.K2_AddActorWorldRotation` _inspectingactor (`KismetMathLibrary.MakeRotator` 0.0 _y _x) false false))
    (:`else`)))

(event `self.ScaleInspectableItem`
  (params (Value :type "InputActionValue Structure (by ref)"))
  (bind _x (`EnhancedInputLibrary.BreakInputActionValue` Value))
  ; Interaction
  ;; Inspect Actions
  (if (`self.CanScaleInInspect` _x)
    (`SceneComponent.K2_AddLocalOffset` (`self.InspectPoint`) (`KismetMathLibrary.MakeVector` _x) false false)))

(event `self.Focus`
  (params (ActorToFocus :type "Actor Object Reference"))
  (bind _returnvalue (`GameplayStatics.GetPlayerController` 0))
  (bind _returnvalue_2 (pcsubsystem `EnhancedInputLocalPlayerSubsystem` _returnvalue))
  ; Interaction
  ;; Focus
  (if (`self.bIsInFocus`)
    (`EnhancedInputSubsystemInterface.ClearAllMappings` _returnvalue_2)
    (`EnhancedInputSubsystemInterface.AddMappingContext` _returnvalue_2 "/Game/Input/Default/IMC_Default.IMC_Default" 0 (struct))
    (`WidgetBlueprintLibrary.SetInputMode_GameOnly` _returnvalue true)
    (set `PlayerController.bShowMouseCursor` false _returnvalue)
    (set `self.bIsInFocus` false)
    (else
      (`EnhancedInputSubsystemInterface.ClearAllMappings` _returnvalue_2)
      (`EnhancedInputSubsystemInterface.AddMappingContext` _returnvalue_2 "/Game/Input/Focus/IMC_Focus.IMC_Focus" 0 (struct))
      (`WidgetBlueprintLibrary.SetInputMode_GameAndUIEx` _returnvalue null "LockAlways" false true)
      (set `PlayerController.bShowMouseCursor` true _returnvalue)
      (set `self.bIsInFocus` true))))

(event `self.ShowInventory`
  (bind _returnvalue (`GameplayStatics.GetPlayerController` 0))
  (bind _returnvalue_2 (pcsubsystem `EnhancedInputLocalPlayerSubsystem` _returnvalue))
  ; Inventory
  (`WidgetBlueprintLibrary.SetInputMode_GameAndUIEx` _returnvalue null "LockAlways" false)
  (set `PlayerController.bShowMouseCursor` true _returnvalue)
  (`EnhancedInputSubsystemInterface.ClearAllMappings` _returnvalue_2)
  (`EnhancedInputSubsystemInterface.AddMappingContext` _returnvalue_2 "/Game/Input/InventoryWidget/IMC_InventoryWidget.IMC_InventoryWidget" 0 (struct))
  (`self.InventoryOpenEventDispatcher` true))

(event `self.HideInventory`
  (bind _returnvalue (`GameplayStatics.GetPlayerController` 0))
  (bind _returnvalue_2 (pcsubsystem `EnhancedInputLocalPlayerSubsystem` _returnvalue))
  ; Inventory
  (`WidgetBlueprintLibrary.SetInputMode_GameOnly` _returnvalue)
  (set `PlayerController.bShowMouseCursor` false _returnvalue)
  (`EnhancedInputSubsystemInterface.ClearAllMappings` _returnvalue_2)
  (`EnhancedInputSubsystemInterface.AddMappingContext` _returnvalue_2 "/Game/Input/Default/IMC_Default.IMC_Default" 0 (struct))
  (`self.InventoryOpenEventDispatcher` false))

(event `self.PauseGame`
  (bind _returnvalue (`GameplayStatics.GetPlayerController` 0))
  (`GameplayStatics.SetGamePaused` true)
  (bind _returnvalue_2 (`|CreateWidget` "/Game/HUD/PauseMenu/WBP_PauseMenu.WBP_PauseMenu_C" _returnvalue))
  (`UserWidget.AddToViewport` _returnvalue_2 0)
  (`WidgetBlueprintLibrary.SetInputMode_GameAndUIEx` _returnvalue null)
  (set `PlayerController.bShowMouseCursor` true _returnvalue))

(fn `CanScaleInInspect`
  (params (Delta :type "Float (double-precision)"))
  (returns (Output :type Boolean))
  (bind _returnvalue (+ Delta (`self.CurrentPointX`)))
  (bind _returnvalue_2 (not (or (< _returnvalue (`self.MInDistance`)) (> _returnvalue (`self.DefaultPointX`)))))
  (if _returnvalue_2
    (set `self.CurrentPointX` _returnvalue)
    (return _returnvalue_2)))

(fn `UserConstructionScript`
  (bind _output_get (set `self.DefaultPointX` (.x (.location (`SceneComponent.GetRelativeTransform` (`self.InspectPoint`))))))
  (set `self.MInDistance` (* _output_get 0.5)))