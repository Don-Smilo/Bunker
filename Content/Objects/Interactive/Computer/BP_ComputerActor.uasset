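; Interactive computer actor that moves the player's view to a camera placed in front of or around it while in use.
; Construction script converts the Arrow component's relative transform into a world-space camera transform.
; StartInteract calls Focus on BP_MainCharacter, spawns a CameraActor there and blends to it.
; StopInteract calls Focus again, blends back to the pawn, then destroys the camera; GetCanInteract blocks re-entry during use.
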(event `InteractableInterface.StartInteract`
  (params (Interactor :type "Actor Object Reference"))
  (bind _asbp_main_character (cast `/Game/Blueprints/BP_MainCharacter` Interactor))
  (`MainCharacter.Focus` _asbp_main_character self)
  (bind _returnvalue (`|SpawnActorFromClass` "/Script/Engine.CameraActor" (`self.CameraTransform`) "Undefined" "MultiplyWithRoot" null null))
  (`PlayerController.SetViewTargetWithBlend` (`GameplayStatics.GetPlayerController` 0) _returnvalue 0.2 "VTBlend_Linear" 0.0 false)
  (set `self.bIsInInteraction` true))

(event `InteractableInterface.StopInteract`
  (params (Interactor :type "Actor Object Reference"))
  (bind _returnvalue (`GameplayStatics.GetPlayerController` 0))
  (bind _asbp_main_character (cast `/Game/Blueprints/BP_MainCharacter` Interactor))
  (`MainCharacter.Focus` _asbp_main_character self)
  (`PlayerController.SetViewTargetWithBlend` _returnvalue (`Controller.K2_GetPawn` _returnvalue) 0.2 "VTBlend_Linear" 0.0 false)
  (`KismetSystemLibrary.Delay` 0.2)
  (`self.K2_DestroyActor` (stale `InteractableInterface.StartInteract` _returnvalue))
  (set `self.bIsInInteraction` false))

(fn `GetCanInteract`
  (returns (ReturnValue :type Boolean))
  (return (not (`self.bIsInInteraction`))))

(fn `UserConstructionScript`
  (bind (_returnvalue_location _returnvalue_rotation) (`KismetMathLibrary.BreakTransform` (`self.GetTransform`)))
  (bind (_returnvalue_location_2 _returnvalue_rotation_2 _returnvalue_scale) (`KismetMathLibrary.BreakTransform` (`SceneComponent.GetRelativeTransform` (`self.Arrow`))))
  (set `self.CameraTransform` (`KismetMathLibrary.MakeTransform` (+ (`KismetMathLibrary.GreaterGreater_VectorRotator` _returnvalue_location_2 _returnvalue_rotation) _returnvalue_location) (`KismetMathLibrary.ComposeRotators` _returnvalue_rotation_2 _returnvalue_rotation) _returnvalue_scale)))