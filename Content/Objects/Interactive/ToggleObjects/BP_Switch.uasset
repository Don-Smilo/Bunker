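; BP_Switch is an interactive switch, a child toggle object whose lever tilts to show its on or off state.
; SetDefaultState snaps the Switch component to the matching roll angle for its initial state.
; Toggle calls the parent logic, plays a Timeline forward or in reverse to animate the roll, then fires the toggle event dispatcher with the new state.
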(event `self.PlayToggleAnimation`
  (params (IsForward :type Boolean))
  (if IsForward
    (bind (_direction _xrotation) (`Timeline|Timeline` :!via `PlayFromStart` :!label _label)
      (:`Update`
        (`SceneComponent.K2_SetRelativeRotation` (`self.switch`) (`KismetMathLibrary.MakeRotator` _xrotation) false false)))
    (else
      (goto _label :!via `ReverseFromEnd`))))

(fn `SetDefaultState`
  (params (IsActive :type Boolean))
  (bind _switch (`self.switch`))
  (`parent.SetDefaultState` IsActive)
  (if IsActive
    (`SceneComponent.K2_SetRelativeRotation` _switch (`KismetMathLibrary.MakeRotator` -17.0) false false)
    (else
      (`SceneComponent.K2_SetRelativeRotation` _switch (`KismetMathLibrary.MakeRotator` 17.0) false false))))

(fn `Toggle`
  (params (Interactor :type "Actor Object Reference") (IsActive :type Boolean))
  (`parent.Toggle` Interactor IsActive)
  (`self.PlayToggleAnimation` IsActive)
  (`self.ToggleEventDispathcer` IsActive))

(fn `UserConstructionScript`
  (`parent.UserConstructionScript`))