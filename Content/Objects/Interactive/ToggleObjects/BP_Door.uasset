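; Interactive door that swings open and closed as a toggle object, overriding its parent's Toggle and SetDefaultState.
; Toggle calls PlayToggleAnimation, which plays a timeline forward when active or in reverse when inactive to drive the Door component's relative yaw.
; SetDefaultState calls the parent, then snaps the door straight to its open (90 degree) or closed yaw without animating.
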(event `self.PlayToggleAnimation`
  (params (IsForward :type Boolean))
  (if IsForward
    (bind (_direction _z_rotation) (`Timeline|Timeline` :!label _label)
      (:`Update`
        (`SceneComponent.K2_SetRelativeRotation` (`self.Door`) (`KismetMathLibrary.MakeRotator` 0.0 0.0 _z_rotation) false false)))
    (else
      (goto _label :!via `Reverse`))))

(fn `SetDefaultState`
  (params (IsActive :type Boolean))
  (bind _door (`self.Door`))
  (`parent.SetDefaultState` IsActive)
  (if IsActive
    (`SceneComponent.K2_SetRelativeRotation` _door (`KismetMathLibrary.MakeRotator` 0.0 0.0 90.0) false false)
    (else
      (`SceneComponent.K2_SetRelativeRotation` _door (`KismetMathLibrary.MakeRotator` 0.0) false false))))

(fn `Toggle`
  (params (Interactor :type "Actor Object Reference") (IsActive :type Boolean))
  (`self.PlayToggleAnimation` IsActive))

(fn `UserConstructionScript`
  (`parent.UserConstructionScript`))