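; BP_Door is an interactive door that swings open and shut when StartInteract is triggered.
; A FlipFlop alternates between playing a timeline from the start and reversing it from the end.
; The timeline's ZRotation track sets the relative yaw of the Cube component.
; BeginPlay, overlap and Tick are unused stubs, so all logic runs from the interact event.
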(event `InteractableInterface.StartInteract`
  (params (Interactor :type "Actor Object Reference"))
  (`/Engine/EditorBlueprintResources/StandardMacros.FlipFlop`
    (:`A`
      (bind (_direction _z_rotation) (`Timeline|Timeline` :!via `PlayFromStart` :!label _label)
        (:`Update`
          (`SceneComponent.K2_SetRelativeRotation` (`self.Cube`) (`KismetMathLibrary.MakeRotator` 0.0 0.0 _z_rotation) false false))))
    (:`B`
      (goto _label :!via `ReverseFromEnd`))))

(fn `UserConstructionScript`
  (`parent.UserConstructionScript`))