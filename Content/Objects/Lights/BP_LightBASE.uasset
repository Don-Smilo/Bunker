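; Base Blueprint for light objects that can be turned on and off by a referenced switch.
; The construction script applies intensity and color to all light components, then sets the default on/off state.
; At BeginPlay it binds to the switch's toggle dispatcher, if one is set, and syncs to its active state.
; Toggling sets intensity to the configured value or zero and calls ToggleMaterial, an empty hook here.
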(event `self.ReceiveBeginPlay`
  (bind _switchref (`self.SwitchRef`))
  (`/Engine/EditorBlueprintResources/StandardMacros.IsValid` _switchref
    (:`Is Valid`
      (add `/Game/Objects/Interactive/ToggleObjects/BP_Switch.ToggleEventDispathcer` _switchref (delegate `Toggle`))
      (bind _output_get (set `self.IsOn` (`/Game/Objects/Interactive/InteractiveBases/InteractableToggleBase.GetIsActive` _switchref)))
      (`self.ToggleLight` _output_get)
      (`self.ToggleMaterial` _output_get))))

(event `Toggle`
  (params (SwitchOn :type Boolean))
  (`self.ToggleLight` SwitchOn)
  (`self.ToggleMaterial` SwitchOn))

(fn `SetLightParams`
  (for _array_element (`self.K2_GetComponentsByClass` "/Script/Engine.LightComponent")
    (`LightComponent.SetIntensity` _array_element (`self.Intensity`))
    (`LightComponent.SetLightColor` _array_element (`self.LightColor`) false)))

(fn `ToggleLight`
  (params (SwitchOn :type Boolean))
  (bind _output_get (set `self.IsOn` SwitchOn))
  (for _array_element (`self.K2_GetComponentsByClass` "/Script/Engine.LightComponent")
    (if _output_get
      (`LightComponent.SetIntensity` _array_element (`self.Intensity`))
      (else
        (`LightComponent.SetIntensity` _array_element 0.0)))))

(fn `ToggleMaterial`
  (params (SwitchOn :type Boolean)))

(fn `UserConstructionScript`
  (`self.SetLightParams`)
  (bind _output_get (set `self.IsOn` (`self.IsOnDefault`)))
  (`self.ToggleLight` _output_get)
  (`self.ToggleMaterial` _output_get))