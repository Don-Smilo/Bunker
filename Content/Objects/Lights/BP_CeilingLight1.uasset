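; BP_CeilingLight1 is a ceiling light Blueprint with a glowing mesh surface that can be switched on and off.
; The construction script creates a dynamic instance of M_GlowingSurface, tints it with LightColor and applies it to the mesh before calling the parent script.
; ToggleMaterial sets the glow parameter from a scaled-down Intensity when on, or to zero when off.
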(event `self.ReceiveBeginPlay`
  (`parent.ReceiveBeginPlay`))

(fn `ToggleMaterial`
  (params (SwitchOn :type Boolean))
  (bind _materialglow (`self.MaterialGlow`))
  (if SwitchOn
    (`MaterialInstanceDynamic.SetScalarParameterValue` _materialglow "Intence" (/ (`self.Intensity`) 1000.0))
    (else
      (`MaterialInstanceDynamic.SetScalarParameterValue` _materialglow "Intence" 0.0))))

(fn `UserConstructionScript`
  (bind _returnvalue (`PrimitiveComponent.CreateDynamicMaterialInstance` (`self.Mesh`) 0 "/Game/Materials/LightMaterials/M_GlowingSurface.M_GlowingSurface" "None"))
  (bind _output_get (set `self.MaterialGlow` _returnvalue))
  (`MaterialInstanceDynamic.SetVectorParameterValue` _output_get "Color" (`self.LightColor`))
  (`PrimitiveComponent.SetMaterial` (`self.Mesh`) 0 (`self.MaterialGlow`))
  (`parent.UserConstructionScript`))